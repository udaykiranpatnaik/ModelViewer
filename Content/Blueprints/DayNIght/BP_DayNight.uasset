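; Day/night lighting switcher that applies one of two preset looks in the construction script or through SetDayNightState, where a true DayNight means night.
; Day and Night configure the referenced directional light and skylight, post-process toggles, moon mesh and a dynamic sky-dome material.
; Both push global material values through MPC_DayNight and toggle root visibility on actors tagged "flare" and "Alula".
; A separate MoonDirection function aligns the moon pivot to the directional light.
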(event EventBeginPlay
  (Class|SkyLightComponent|RecaptureSky (Variables|/Script/Engine.SkyLight|GetLightComponent (Variables|Default|GetSkylightSelection))))

(fn ConstructionScript
  (Class|SkyLightComponent|RecaptureSky (Variables|/Script/Engine.SkyLight|GetLightComponent (Variables|Default|GetSkylightSelection)))
  (if (Variables|Default|GetDay/Night)
    (CallFunction|Night)
    (else
      (CallFunction|Day))))

(fn Day
  (bind _directional_light (Variables|Default|GetDirectional%20Light))
  (bind _skylightselection (Variables|Default|GetSkylightSelection))
  (bind _lightcomponent (Variables|/Script/Engine.Light|GetLightComponent _directional_light))
  (bind _lightcomponent_2 (Variables|/Script/Engine.SkyLight|GetLightComponent _skylightselection))
  (bind _lightcomponent_3 (Variables|/Script/Engine.Light|GetLightComponent _directional_light))
  ;[1 1 1] Visibility Parameters for Day/Night
  (Rendering|SetVisibility (Variables|Components|GetSM_Moon) false false)
  (Variables|/Script/Engine.PostProcessVolume|SetbEnabled (Variables|Default|Getpp_night) false)
  (Variables|/Script/Engine.PostProcessVolume|SetbEnabled (Variables|Default|Getpp_day) true)
  (if (Variables|Day|GetLight%20Temp%20Day)
    (Class|LightComponent|SetUseTemperature _lightcomponent true)
    (Class|LightComponent|SetTemperature _lightcomponent_3 (Variables|Day|GetDay%20Light%20Temp))
    (else
      (Class|LightComponent|SetUseTemperature _lightcomponent false)))
  (Transformation|SetActorLocationAndRotation _directional_light "0, 0, 0" "-48.651154,82.464409,-1.548629")
  ;[1 1 1] Directional Light Properties
  (Class|DirectionalLightComponent|SetShadowAmount (Actor|GetComponentbyClass _directional_light "/Script/Engine.DirectionalLightComponent") 1.0)
  (Rendering|Components|Light|SetIntensity _lightcomponent_3 (Variables|Day|GetDL%20Intensity%20Day))
  (Rendering|Components|Light|SetLightColor _lightcomponent_3 (Variables|Day|GetDay%20Light%20Color) true)
  (Class|SkyLightComponent|SetLowerHemisphereColor _lightcomponent_2 (Variables|Default|GetIn%20Lower%20Hemisphere%20Color_0))
  ;[1 1 1] SkyLight Parameters
  (Rendering|Components|Light|SetIntensity _lightcomponent_2 (Variables|Day|GetSelect%20Light%20Intensity%20Day))
  (Class|SkyLightComponent|RecaptureSky _lightcomponent_2)
  (Class|SkyLightComponent|SetCubemap _lightcomponent_2 (Variables|Day|GetSet%20SkyLight%20Day%20HDR))
  ;[1 1 1] Updates for the Materials
  (bind _returnvalue (Rendering|Material|CreateDynamicMaterialInstance (Variables|Components|GetSM_EnvDome) 0 "/Game/Blueprints/DayNIght/Assets/Materials/M_Skybox.M_Skybox" "None" :!class /Script/Engine.PrimitiveComponent))
  (Rendering|Material|SetScalarParameterValue _returnvalue "Intensity" (Variables|Day|GetSky%20Intensity%20Day) :!class /Script/Engine.MaterialInstanceDynamic)
  (Rendering|Material|SetTextureParameterValue _returnvalue "SelectHDR" (Variables|Day|GetSelect%20Day%20HDR))
  (Rendering|Material|SetScalarParameterValue "/Game/Blueprints/DayNIght/Assets/MPC/MPC_DayNight.MPC_DayNight" "Diffuse_Brightness" (Variables|Day|GetDiffuse%20Brightness) :!class /Script/Engine.KismetMaterialLibrary)
  (Rendering|Material|SetScalarParameterValue "/Game/Blueprints/DayNIght/Assets/MPC/MPC_DayNight.MPC_DayNight" "IsEmissive" 0.0 :!class /Script/Engine.KismetMaterialLibrary)
  (Rendering|Material|SetScalarParameterValue "/Game/Blueprints/DayNIght/Assets/MPC/MPC_DayNight.MPC_DayNight" "LightTemp" 0.0 :!class /Script/Engine.KismetMaterialLibrary)
  (Rendering|Material|SetScalarParameterValue "/Game/Blueprints/DayNIght/Assets/MPC/MPC_DayNight.MPC_DayNight" "Glass" 1.0 :!class /Script/Engine.KismetMaterialLibrary)
  (Rendering|Material|SetScalarParameterValue "/Game/Blueprints/DayNIght/Assets/MPC/MPC_DayNight.MPC_DayNight" "Road Brightness" 1.0 :!class /Script/Engine.KismetMaterialLibrary)
  (Rendering|Material|SetScalarParameterValue "/Game/Blueprints/DayNIght/Assets/MPC/MPC_DayNight.MPC_DayNight" "Character Shadow Plane Opacity" 1.0 :!class /Script/Engine.KismetMaterialLibrary)
  (Rendering|Material|SetScalarParameterValue "/Game/Blueprints/DayNIght/Assets/MPC/MPC_DayNight.MPC_DayNight" "Bright Billboard" 1.0 :!class /Script/Engine.KismetMaterialLibrary)
  (Utilities|FlowControl|Sequence
    (:then_0
      (bind _outactors (Actor|GetAllActorswithTag "flare"))
      (for _array_element _outactors
        (Rendering|SetVisibility (Variables|/Script/Engine.Actor|GetRootComponent _array_element) false false)))
    (:then_1
      (bind _outactors_2 (Actor|GetAllActorswithTag "Alula"))
      (for _array_element_2 _outactors_2
        (Rendering|SetVisibility (Variables|/Script/Engine.Actor|GetRootComponent _array_element_2) true false)))))

(fn Night
  (bind _sm_moon (Variables|Components|GetSM_Moon))
  (bind _directional_light (Variables|Default|GetDirectional%20Light))
  (bind _skylightselection (Variables|Default|GetSkylightSelection))
  (bind _moonscale (Variables|Night|GetMoonScale))
  (bind _lightcomponent (Variables|/Script/Engine.Light|GetLightComponent _directional_light))
  (bind _lightcomponent_2 (Variables|/Script/Engine.Light|GetLightComponent _directional_light))
  (bind _lightcomponent_3 (Variables|/Script/Engine.SkyLight|GetLightComponent _skylightselection))
  ;[1 1 1] Visibility Parameters for Day/Night
  (Rendering|SetVisibility (Variables|Components|GetSM_Moon) true false)
  (Variables|/Script/Engine.PostProcessVolume|SetbEnabled (Variables|Default|Getpp_night) true)
  (Variables|/Script/Engine.PostProcessVolume|SetbEnabled (Variables|Default|Getpp_day) false)
  ;[1 1 1] Moon Parameters
  (Transformation|SetWorldScale3D _sm_moon (Math|Vector|MakeVector _moonscale _moonscale _moonscale))
  (Rendering|Material|SetScalarParameterValueonMaterials _sm_moon "Moon_Emission" (Variables|Night|GetMoon%20Glow))
  (if (Variables|Night|GetLight%20Temp%20Night)
    (Class|LightComponent|SetUseTemperature _lightcomponent true)
    (Class|LightComponent|SetTemperature _lightcomponent_2 (Variables|Night|GetNight%20DL%20Temp))
    (else
      (Class|LightComponent|SetUseTemperature _lightcomponent false)))
  (Transformation|SetActorLocationAndRotation _directional_light "0, 0, 0" (Variables|Default|GetMoon%20Rotation))
  ;[1 1 1] Directional Light
  (Rendering|Components|Light|SetIntensity _lightcomponent_2 (Variables|Night|GetDL%20Intensity%20Night))
  (Rendering|Components|Light|SetLightColor _lightcomponent_2 (Variables|Night|GetNight%20Light%20Color) true)
  (Class|DirectionalLightComponent|SetShadowAmount (Actor|GetComponentbyClass _directional_light "/Script/Engine.DirectionalLightComponent") 0.3)
  ;[1 1 1] SkyLight Parameters
  (Class|SkyLightComponent|SetLowerHemisphereColor _lightcomponent_3 (Variables|Default|GetIn%20Lower%20Hemisphere%20Color))
  (Rendering|Components|Light|SetLightColor _lightcomponent_3 (Variables|Night|GetSkyLight_Color%28Night%29))
  (Rendering|Components|Light|SetIntensity _lightcomponent_3 (Variables|Night|GetSelect%20Light%20Intensity%20Night))
  (Class|SkyLightComponent|RecaptureSky _lightcomponent_3)
  (Class|SkyLightComponent|SetCubemap _lightcomponent_3 (Variables|Night|GetSelect%20Night%20HDR))
  ;[1 1 1] Material Parameters
  (bind _returnvalue (Rendering|Material|CreateDynamicMaterialInstance (Variables|Components|GetSM_EnvDome) 0 "/Game/Blueprints/DayNIght/Assets/Materials/M_Skybox.M_Skybox" "None" :!class /Script/Engine.PrimitiveComponent))
  (Rendering|Material|SetScalarParameterValue _returnvalue "Intensity" (Variables|Night|GetSky%20Intensity%20Night) :!class /Script/Engine.MaterialInstanceDynamic)
  (Rendering|Material|SetTextureParameterValue _returnvalue "SelectHDR" (Variables|Night|GetSelect%20Night%20HDR))
  (Rendering|Material|SetScalarParameterValue "/Game/Blueprints/DayNIght/Assets/MPC/MPC_DayNight.MPC_DayNight" "Diffuse_Brightness" (Variables|Night|GetDiffuse%20Brightness%20Night) :!class /Script/Engine.KismetMaterialLibrary)
  (Rendering|Material|SetScalarParameterValue "/Game/Blueprints/DayNIght/Assets/MPC/MPC_DayNight.MPC_DayNight" "IsEmissive" (Variables|Night|GetGlow%20Value) :!class /Script/Engine.KismetMaterialLibrary)
  (Rendering|Material|SetScalarParameterValue "/Game/Blueprints/DayNIght/Assets/MPC/MPC_DayNight.MPC_DayNight" "LightTemp" (Variables|Night|GetEmission%20Light%20Temp) :!class /Script/Engine.KismetMaterialLibrary)
  (Rendering|Material|SetScalarParameterValue "/Game/Blueprints/DayNIght/Assets/MPC/MPC_DayNight.MPC_DayNight" "Bright Billboard" (Variables|Night|GetBrightness%20Billboard) :!class /Script/Engine.KismetMaterialLibrary)
  (Rendering|Material|SetScalarParameterValue "/Game/Blueprints/DayNIght/Assets/MPC/MPC_DayNight.MPC_DayNight" "Glass" (Variables|Default|GetGlass%20Night) :!class /Script/Engine.KismetMaterialLibrary)
  (Rendering|Material|SetScalarParameterValue "/Game/Blueprints/DayNIght/Assets/MPC/MPC_DayNight.MPC_DayNight" "Road Brightness" (Variables|Night|GetRoad%20Brightness) :!class /Script/Engine.KismetMaterialLibrary)
  (Rendering|Material|SetScalarParameterValue "/Game/Blueprints/DayNIght/Assets/MPC/MPC_DayNight.MPC_DayNight" "Character Shadow Plane Opacity" (Variables|Night|GetCharacter%20Fake%20Shadow%20Opacity) :!class /Script/Engine.KismetMaterialLibrary)
  (Utilities|FlowControl|Sequence
    (:then_0
      (bind _outactors (Actor|GetAllActorswithTag "flare"))
      (for _array_element _outactors
        (Rendering|SetVisibility (Variables|/Script/Engine.Actor|GetRootComponent _array_element) true false)))
    (:then_1
      (bind _outactors_2 (Actor|GetAllActorswithTag "Alula"))
      (for _array_element_2 _outactors_2
        (Rendering|SetVisibility (Variables|/Script/Engine.Actor|GetRootComponent _array_element_2) false false)))))

(fn MoonDirection
  (Transformation|SetRelativeRotation (Variables|Components|GetMoonPivot) (.rotation (Transformation|GetRelativeTransform (Variables|/Script/Engine.Light|GetLightComponent (Variables|Default|GetDirectional%20Light)))) false false))

(fn SetDayNightState
  (params (Condition :type Boolean))
  (bind _output_get (Variables|Default|SetDay/Night Condition))
  (Class|SkyLightComponent|RecaptureSky (Variables|/Script/Engine.SkyLight|GetLightComponent (Variables|Default|GetSkylightSelection)))
  (if _output_get
    (CallFunction|Night)
    (else
      (CallFunction|Day))))